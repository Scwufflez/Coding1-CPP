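; A falling platform that drops shortly after the custom third-person character enters its trigger box, then returns to its start.
; Activation locks retriggering and waits briefly, then Drop enables physics on the cube, and after a further delay Reset disables it.
; A timeline lerps the cube from where it fell back to the transform saved at BeginPlay, then re-arms it.
; The cube's material changes with each state.
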(event OnComponentBeginOverlap(Box)
  (params (OverlappedComponent :type Primitive%20Component%20Object%20Reference) (OtherActor :type Actor%20Object%20Reference) (OtherComp :type Primitive%20Component%20Object%20Reference) (OtherBodyIndex :type Integer) (bFromSweep :type Boolean) (SweepResult :type Hit%20Result%20Structure%20%28by%20ref%29))
  (Utilities|Casting|CastToBP_ThirdPersonCharacterCustom OtherActor)
  (CallFunction|Activate))

(event Custom|Activate
  (if (Variables|Default|Getready)
    (Development|PrintString "one secoond left!")
    (Variables|Default|Setready false)
    (Rendering|Material|SetMaterial (Variables|Default|GetCube) 0 "/Game/Materials/PlatformActivated.PlatformActivated")
    (Utilities|FlowControl|Delay 1.0)
    (CallFunction|Drop)))

(event Custom|Drop
  (Development|PrintString "Dropping!")
  (Physics|SetSimulatePhysics (Variables|Default|GetCube) true)
  (Rendering|Material|SetMaterial (Variables|Default|GetCube) 0 "/Game/Materials/PlatformFalling.PlatformFalling")
  (Utilities|FlowControl|Delay 3.0)
  (CallFunction|Reset))

(event Custom|Reset
  (Development|PrintString "Resetting!")
  (Variables|Default|SetResetTransform (Transformation|GetWorldTransform (Variables|Default|GetCube)))
  (Physics|SetSimulatePhysics (Variables|Default|GetCube) false)
  (Rendering|Material|SetMaterial (Variables|Default|GetCube) 0 "/Game/Materials/PlatformRestting.PlatformRestting")
  (bind _float (Timeline|GobacktoStart PlayFromStart)
    (:Update
      (Transformation|SetWorldLocationAndRotation (Variables|Default|GetCube) (.location (Math|Transform|Lerp(Transform) (Variables|Default|GetResetTransform) (Variables|Default|GetStarting%20transform) _float)) (.rotation (Math|Transform|Lerp(Transform) (Variables|Default|GetResetTransform) (Variables|Default|GetStarting%20transform) _float)) false false))
    (:Finished
      (Variables|Default|Setready true)
      (Rendering|Material|SetMaterial (Variables|Default|GetCube) 0 "/Game/Materials/MI_PlatformReady.MI_PlatformReady"))))

(event EventBeginPlay
  (Variables|Default|SetStarting%20transform (Transformation|GetWorldTransform (Variables|Default|GetCube)))
  (Rendering|Material|SetMaterial (Variables|Default|GetCube) 0 "/Game/Materials/MI_PlatformReady.MI_PlatformReady"))

(event Collision|EventActorBeginOverlap
  (params (OtherActor :type Actor%20Object%20Reference)))

(event EventTick
  (params (DeltaSeconds :type Float%20%28single-precision%29)))

(fn ConstructionScript)